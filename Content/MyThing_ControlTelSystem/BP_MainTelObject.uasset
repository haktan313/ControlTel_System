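; Telekinesis object actor that a player can hold, spin, release or throw.
; Once LaunchItem sets the player and launch flag, Tick lerps the actor to an offset beside the player with Object physics simulation off.
; RotateLaunch adds smoothed roll and yaw, while ReleaseItem restores physics.
; ThrowItem ends the hold and applies a clamped-speed impulse toward the target, or along the player's forward vector without one.
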(event EventTick
  (params (DeltaSeconds :type Float%20%28single-precision%29))
  (bind _player (Variables|Default|GetPlayer))
  ;[0 0 0 0.786] SetPositionOfItem
  (if (Variables|Default|GetCan%20Launch)
    (Transformation|SetActorLocation (Math|Vector|Lerp(Vector) (Transformation|GetActorLocation self) (+ (+ (Transformation|GetActorLocation _player) "45.000000,0.000000,65.000000") (* (Transformation|GetActorRightVector _player) -1.5e+02)) 0.08) false false)
    (Physics|SetSimulatePhysics (Variables|Default|Getobject) false)
    (Collision|SetCollisionEnabled (Variables|Default|Getobject) "PhysicsOnly")))

(event EventLaunchItem
  (params (player :type Actor%20Object%20Reference) (canLaunch :type Boolean))
  (Variables|Default|SetPlayer player)
  (Variables|Default|SetCan%20Launch canLaunch))

(event EventThrowItem
  (params (throwTarget :type Actor%20Object%20Reference) (throwSpeed :type Float%20%28double-precision%29))
  ;[0 0 0] Throw
  (if (Variables|Default|GetCan%20Launch)
    (Variables|Default|SetThrow%20Target throwTarget)
    (Variables|Default|SetThrow%20Speed (Math|Float|Clamp(Float) throwSpeed 0.0 (Variables|speed|GetmaxThrowSpeed)))
    (Physics|SetSimulatePhysics (Variables|Default|Getobject) true)
    (Collision|SetCollisionEnabled (Variables|Default|Getobject) "QueryAndPhysics")
    (Variables|Default|SetCan%20Launch false)
    (Utilities|IsValid (Variables|Default|GetThrow%20Target)
      (:Is%20Valid
        (Physics|AddImpulseatLocation (Variables|Default|Getobject) (* (Math|Vector|Normalize (- (Transformation|GetActorLocation (Variables|Default|GetThrow%20Target)) (Transformation|GetActorLocation))) 222222.0 (Variables|Default|GetThrow%20Speed)) (Transformation|GetActorLocation) "None"))
      (:Is%20Not%20Valid
        (bind _player (Variables|Default|GetPlayer)
          (:then
            (Physics|AddImpulseatLocation (Variables|Default|Getobject) (* (Transformation|GetActorForwardVector _player) 222222.0 (Variables|Default|GetThrow%20Speed)) (Transformation|GetActorLocation) "None"))
          (:else))))))

(event EventReleaseItem
  (bind _object (Variables|Default|Getobject)
    (:then
      (Physics|SetSimulatePhysics _object true)
      (Collision|SetCollisionEnabled _object "QueryAndPhysics"))
    (:else)))

(event EventRotateLaunch
  (bind _returnvalue (Transformation|GetActorRotation))
  (if (Variables|Default|GetCan%20Launch)
    (Transformation|SetActorRotation (Math|Rotator|Lerp(Rotator) (Transformation|GetActorRotation) (Math|Rotator|MakeRotator (+ (.roll _returnvalue) 12.0) (+ (.pitch _returnvalue) 0.0) (+ (.yaw _returnvalue) 12.0)) 0.4))))

(fn ConstructionScript)